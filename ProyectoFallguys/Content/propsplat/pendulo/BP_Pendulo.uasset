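; BP_Pendulo is a swinging pendulum obstacle that knocks the player away.
; From BeginPlay, a looping three-second timer alternates a timeline between play and reverse through a FlipFlop, lerping the static mesh's relative rotation between start and end rotations.
; Any actor overlap launches player character 0 along world +Y, overriding horizontal velocity, and plays a 2D hit sound only the first time.
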(event `self.ReceiveBeginPlay`
  (`self.RotatePendulo`)
  (`KismetSystemLibrary.K2_SetTimerDelegate` (delegate `RotatePendulo`) 3.0 true 0.1))

(event `RotatePendulo`
  (`/Engine/EditorBlueprintResources/StandardMacros.FlipFlop`
    (:`A`
      (bind (_direction _pendulorot) (`Timeline|PenduloRotation` :!label _label)
        (:`Update`
          (`SceneComponent.K2_SetRelativeRotation` (`self.StaticMesh`) (`KismetMathLibrary.RLerp` (`self.StartRotation`) (`self.EndRotation`) _pendulorot) false false))))
    (:`B`
      (goto _label :!via `Reverse`))))

(event `self.ReceiveActorBeginOverlap`
  (params (OtherActor :type "Actor Object Reference"))
  (`Character.LaunchCharacter` (`GameplayStatics.GetPlayerCharacter` 0) (0.0 1000.0 0.0) true false)
  (`/Engine/EditorBlueprintResources/StandardMacros.DoOnce` false
    (:`Completed`
      (`GameplayStatics.PlaySound2D` "/Game/StarterContent/Audio/hit_fall.hit_fall" 1.0 1.0 0.0 null null))))

(fn `UserConstructionScript`)